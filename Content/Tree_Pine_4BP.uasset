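; Felled pine tree actor that topples as a physics object and then turns into inventory items for the player.
; On BeginPlay it sets mass by world scale and pushes itself along the player camera's forward vector with a scaled impulse.
; After a short delay, item quantity follows Z scale, and Tick watches for zero velocity.
; Once still, it waits, destroys itself and adds the item plus proportional Sticks to the inventory widget.
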(event `self.ReceiveBeginPlay`
  (bind _sm_pine_tree_4 (`self.SM_Pine_Tree_4`))
  (bind _returnvalue (/ (.x (`SceneComponent.K2_GetComponentScale` (`self.SM_Pine_Tree_4`))) 10.0))
  (bind _returnvalue_2 (`GameplayStatics.GetActorOfClass` "/Game/FirstPersonCPP/Blueprints/FirstPersonCharacter.FirstPersonCharacter_C"))
  (`PrimitiveComponent.SetMassOverrideInKg` _sm_pine_tree_4 "None" (* _returnvalue (`PrimitiveComponent.GetMass` _sm_pine_tree_4)) true)
  (`PrimitiveComponent.AddImpulse` (`self.SM_Pine_Tree_4`) (* (`SceneComponent.GetForwardVector` (`GraCharacter.FirstPersonCameraComponent` _returnvalue_2)) (* 300000 _returnvalue)) "None" false)
  (`KismetSystemLibrary.Delay` 3.0)
  (bind _structout (setmembers `/Game/Migrate/ItemInfoStructure` :`StructRef` (`self.ItemInfo`) :`Quantity` (`KismetMathLibrary.Round` (.z (`SceneComponent.K2_GetComponentScale` (`self.SM_Pine_Tree_4`))))))
  (set `self.ItemInfo` _structout)
  (set `self.Begin` true))

(event `self.ReceiveTick`
  (params (DeltaSeconds :type "Float (single-precision)"))
  (bind _iteminfo (`self.ItemInfo`))
  (bind _returnvalue (`PrimitiveComponent.GetPhysicsLinearVelocity` (`self.SM_Pine_Tree_4`) "None"))
  (if (and (== _returnvalue (0.0 0.0 0.0) :`ErrorTolerance` 0.0) (`self.Begin`))
    (`KismetSystemLibrary.Delay` 10.0)
    (`self.K2_DestroyActor`)
    (bind _asfirst_person_character (cast `/Game/FirstPersonCPP/Blueprints/FirstPersonCharacter` (`GameplayStatics.GetPlayerCharacter` 0)))
    (bind _inventorywidget (`/Game/FirstPersonCPP/Blueprints/FirstPersonCharacter.InventoryWidget` _asfirst_person_character))
    (`/Game/Migrate/UI/Inventory.AddToInventory` _inventorywidget _iteminfo)
    (`/Game/Migrate/UI/Inventory.AddToInventory` _inventorywidget (make `/Game/Migrate/ItemInfoStructure` "Stick" "/Game/Migrate/Items/stick.stick" "Stick" (`KismetMathLibrary.Round` (* (`.Quantity_16_239B480C49901E883690F78625348B18` (break `/Game/Migrate/ItemInfoStructure` _iteminfo)) 1.5))))))

(fn `UserConstructionScript`)